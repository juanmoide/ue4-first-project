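; Enemy character Blueprint that handles damage, hit reactions and death.
; ApplyDamage takes the hit bone: a head hit kills instantly, while other hits subtract health and kill at zero.
; Surviving hits play a damage sound, briefly slow movement and silence Screaming, both restored by a retriggerable delay.
; Death stops Screaming and movement, turns the mesh into a physics ragdoll without capsule collision, then destroys the actor after a delay.
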(event Custom|Apply%20Damage
  (params (Bone :type Name))
  (bind _charactermovement (Variables|Character|GetCharacterMovement))
  ;[1 1 1] Gestiona la vida y la muerte del enemigo
  (if (not (Variables|Default|Getdead))
    (if (Utilities|Name|Equal(Name) Bone "head")
      (Variables|Default|Setdead true :!label _label)
      (Utilities|FlowControl|Sequence
        (:then_0
          (Components|Activation|Deactivate (Variables|Default|GetScreaming)))
        (:then_1
          (CallFunction|SimulateDeathRagdoll Bone)
          (Utilities|FlowControl|Delay 3.0)
          (Actor|DestroyActor)))
      (else
        (bind _output_get (Variables|Default|Sethealth (- (Variables|Default|Gethealth) 5e+01)))
        (if (<= _output_get 0.0)
          (goto _label)
          (else
            (Variables|/Script/Engine.CharacterMovementComponent|SetMaxWalkSpeed _charactermovement 2e+02)
            (Utilities|FlowControl|Sequence
              (:then_0
                (Utilities|FlowControl|RetriggerableDelay 1.0)
                (Utilities|FlowControl|Sequence
                  (:then_0
                    (Variables|/Script/Engine.CharacterMovementComponent|SetMaxWalkSpeed _charactermovement 8e+02))
                  (:then_1
                    (if (not (Variables|Default|Getdead))
                      (Components|Activation|Activate (Variables|Default|GetScreaming) false)))))
              (:then_1
                (Components|Activation|Deactivate (Variables|Default|GetScreaming)))
              (:then_2
                (Audio|PlaySoundatLocation "/Game/StarterContent/Audio/damage.Damage" (Transformation|GetActorLocation))))))))))

(fn ConstructionScript)

(fn SimulateDeathRagdoll
  (params (bone :type Name))
  (bind _mesh (Variables|Character|GetMesh))
  (Pawn|Components|CharacterMovement|DisableMovement (Variables|Character|GetCharacterMovement))
  (Utilities|FlowControl|Sequence
    (:then_0
      (Collision|SetCollisionEnabled (Variables|Collision|GetCapsuleComponent) "NoCollision"))
    (:then_1
      (Collision|SetCollisionEnabled _mesh "PhysicsOnly")
      (Collision|SetCollisionProfileName _mesh bone :!class /Script/Engine.PrimitiveComponent)
      (Physics|SetSimulatePhysics _mesh true))))